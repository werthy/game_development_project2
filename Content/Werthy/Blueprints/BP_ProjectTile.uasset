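; BP_ProjectTile is a projectile that damages characters, scores hits and destroys itself a second after impact.
; On Hit, it filters for blocking GameTraceChannel1, non-projectile actors and an IsValid flag, which allows one effective hit.
; Player characters other than the owner and AI characters lose health.
; Other hits increment the owning character's score, update its HUD and push physics-simulating components with a velocity-based impulse.
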(event `self.ReceiveHit`
  (params (MyComp :type "PrimitiveComponent Object Reference") (Other :type "Actor Object Reference") (OtherComp :type "PrimitiveComponent Object Reference") (bSelfMoved :type Boolean) (HitLocation :type "Vector Structure") (HitNormal :type "Vector Structure") (NormalImpulse :type "Vector Structure") (Hit :type "HitResult Structure (by ref)"))
  (bind _other_comp (`self.Other Comp`))
  (set `self.Other` Other)
  (set `self.Other Comp` OtherComp)
  (if (and (`|EnumEquality` (`PrimitiveComponent.GetCollisionResponseToChannel` OtherComp "ECC_GameTraceChannel1") "ECR_Block") (!= (`GameplayStatics.GetObjectClass` (`self.Other`)) "BP_ProjectTile_C") (`self.bIsValid`))
    (if (== (`GameplayStatics.GetObjectClass` (`self.Other`)) "/Game/Werthy/Blueprints/BP_ThirdPersonCharacter.BP_ThirdPersonCharacter_C")
      (bind _asbp_third_person_character (cast `/Game/Werthy/Blueprints/BP_ThirdPersonCharacter` (`self.Other`)))
      (if (not (== _asbp_third_person_character (`self.GetOwner`)))
        (set `/Game/Werthy/Blueprints/BP_ThirdPersonCharacter.iHealth` (- (`/Game/Werthy/Blueprints/BP_ThirdPersonCharacter.iHealth` _asbp_third_person_character) 10) _asbp_third_person_character))
      (elif (== (`GameplayStatics.GetObjectClass` (`self.Other`)) "/Game/Werthy/Blueprints/AI/BP_AICharacter.BP_AICharacter_C")
        (bind _asbp_aicharacter (cast `/Game/Werthy/Blueprints/AI/BP_AICharacter` (`self.Other`)))
        (set `/Game/Werthy/Blueprints/AI/BP_AICharacter.iHealth` (- (`/Game/Werthy/Blueprints/AI/BP_AICharacter.iHealth` _asbp_aicharacter) 10) _asbp_aicharacter)
        (else
          (`KismetSystemLibrary.PrintString` "Hello")
          (bind _asbp_third_person_character_2 (cast `/Game/Werthy/Blueprints/BP_ThirdPersonCharacter` (`self.GetOwner`)))
          (bind _result (`/Engine/EditorBlueprintResources/StandardMacros.IncrementInt` (`/Game/Werthy/Blueprints/BP_ThirdPersonCharacter.Score` _asbp_third_person_character_2))
            (:`  `
              (message `/Game/Werthy/Blueprints/BP_ScoreInterface.IScoreEvent` (`/Game/Werthy/Blueprints/BP_ThirdPersonCharacter.ThirdPersonHUDRef` _asbp_third_person_character_2) _result)
              (if (`SceneComponent.IsSimulatingPhysics` _other_comp "None")
                (`PrimitiveComponent.AddImpulseAtLocation` _other_comp (* (`self.GetVelocity`) 100.0) (`self.K2_GetActorLocation`) "None")))))))
    (set `self.bIsValid` false))
  (`KismetSystemLibrary.Delay` 1.0)
  (`self.K2_DestroyActor`))

(fn `UserConstructionScript`)