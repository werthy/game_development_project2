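; Networked AI enemy character that detects the third-person player, shoots at them and dies when its health runs out.
; On authority, AI perception writes whether the player is sensed to a blackboard flag.
; AI_Fire line-traces from a muzzle sphere along the gun's rotated forward vector, subtracts player health on hit and triggers client-side montage and sound.
; The health OnRep updates a color-coded text display and starts the death montage and destruction at zero.
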(event `AI_Fire`
  (bind _returnvalue (`SceneComponent.K2_GetComponentLocation` (`self.Sphere`)))
  (bind (_outhit _returnvalue_2) (`KismetSystemLibrary.LineTraceSingle` :`Start` _returnvalue :`End` (+ _returnvalue (* (`KismetMathLibrary.GreaterGreater_VectorRotator` (`SceneComponent.GetForwardVector` (`self.ColorfunGun`)) (struct :`Yaw` 90.0)) 1000.0)) :`TraceChannel` "TraceTypeQuery3" :`DrawDebugType` "ForDuration"))
  (`self.FireEvent_Client`)
  (if _returnvalue_2
    (bind _asbp_third_person_character (cast `/Game/Werthy/Blueprints/BP_ThirdPersonCharacter` (`.HitActor` (`GameplayStatics.BreakHitResult` _outhit))))
    (set `/Game/Werthy/Blueprints/BP_ThirdPersonCharacter.iHealth` (- (`/Game/Werthy/Blueprints/BP_ThirdPersonCharacter.iHealth` _asbp_third_person_character) 5) _asbp_third_person_character)))

(event `FireEvent_Client`
  (`AnimInstance.Montage_Play` (`SkeletalMeshComponent.GetAnimInstance` (`self.Mesh`)) "/Game/Werthy/Animations/Fire_Thirdperson.Fire_Thirdperson" 1.0 "MontageLength" 0.0 true)
  (`GameplayStatics.PlaySoundAtLocation` "/Game/FirstPerson/Audio/FirstPersonTemplateWeaponFire02.FirstPersonTemplateWeaponFire02" (`self.K2_GetActorLocation`) (struct) 0.5 1.0 0.0 null null null))

(event `self.AIPerception.OnTargetPerceptionUpdated`
  (params (Actor :type "Actor Object Reference") (Stimulus :type "AIStimulus Structure"))
  (bind (_age _expirationage _strength _stimuluslocation _receiverlocation _tag _bsuccessfullysensed) (break `AIStimulus` Stimulus))
  (bind _returnvalue (`AIBlueprintHelperLibrary.GetBlackboard` null))
  (`/Engine/EditorBlueprintResources/ActorMacros.Switch Has Authority`
    (:`Authority`
      (if (== (`GameplayStatics.GetObjectClass` Actor) "/Game/Werthy/Blueprints/BP_ThirdPersonCharacter.BP_ThirdPersonCharacter_C")
        (if (== (`BlackboardComponent.GetValueAsBool` _returnvalue "bHasFoundPlayer") (not _bsuccessfullysensed))
          (`BlackboardComponent.SetValueAsBool` _returnvalue "bHasFoundPlayer" _bsuccessfullysensed)
          (`KismetSystemLibrary.PrintString` (`KismetStringLibrary.Conv_BoolToString` _bsuccessfullysensed)))))))

(event `DeathEvent_Server`
  (`self.DeathEvent_Client`))

(event `DeathEvent_Client`
  (bind _returnvalue (`AnimInstance.Montage_Play` (`SkeletalMeshComponent.GetAnimInstance` (`self.Mesh`)) "/Game/Werthy/Animations/Death_ThirdPerson.Death_ThirdPerson" 1.0 "MontageLength" 0.0 true))
  (`KismetSystemLibrary.Delay` (- _returnvalue 0.3))
  (`self.K2_DestroyActor`))

(fn `OnRep_iHealth`
  (bind _ihealth (`self.iHealth`))
  (bind _health (`self.Health`))
  (`TextRenderComponent.K2_SetText` (`self.Health`) (`KismetTextLibrary.Conv_IntToText` _ihealth))
  (if (> _ihealth 20)
    (`TextRenderComponent.SetTextRenderColor` _health (make `Color` 255 255 0 255))
    (else
      (`TextRenderComponent.SetTextRenderColor` _health (make `Color` 0 0 255 255))
      (if (<= (`self.iHealth`) 0)
        (`self.DeathEvent_Server`)))))

(fn `UserConstructionScript`
  (`parent.UserConstructionScript`))