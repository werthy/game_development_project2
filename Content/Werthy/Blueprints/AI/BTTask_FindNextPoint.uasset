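; Behavior tree task that steps an AI along the level's BP_NavSpline path, one spline point at a time.
; It writes the world location of the point at blackboard key iSplineIndex into targetPosition, then increments the index, wrapping to the start after the last point.
; The spline is found with GetActorOfClass on each execution, and the task fails if none exists.
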(event `self.ReceiveExecute`
  (params (OwnerActor :type "Actor Object Reference"))
  (bind _returnvalue (`AIBlueprintHelperLibrary.GetBlackboard` OwnerActor))
  (bind _returnvalue_2 (`BlackboardComponent.GetValueAsInt` _returnvalue "iSplineIndex"))
  (bind _returnvalue_3 (`GameplayStatics.GetActorOfClass` "/Game/Werthy/Blueprints/AI/BP_NavSpline.BP_NavSpline_C"))
  (`/Engine/EditorBlueprintResources/StandardMacros.IsValid` _returnvalue_3
    (:`Is Valid`
      (bind _spline (`/Game/Werthy/Blueprints/AI/BP_NavSpline.Spline` _returnvalue_3))
      (`BlackboardComponent.SetValueAsVector` _returnvalue "targetPosition" (`SplineComponent.GetLocationAtSplinePoint` _spline _returnvalue_2 "World"))
      (`BlackboardComponent.SetValueAsInt` _returnvalue "iSplineIndex" (mod (+ _returnvalue_2 1) (`SplineComponent.GetNumberOfSplinePoints` _spline)))
      (`self.FinishExecute` true))
    (:`Is Not Valid`
      (`self.FinishExecute` false))))