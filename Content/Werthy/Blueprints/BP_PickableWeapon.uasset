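; Pickable weapon actor that a third-person character can pick up while standing in its pickup area.
; Overlapping PickableArea registers the weapon as the character's interaction object and opens a gate; leaving clears the reference and closes it.
; The server pickup event passes through that gate to the client event, which only hides the ColorfulWeapon component, with no inventory or equip logic here.
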(event `InputPickUpEvent_Server`
  (`/Engine/EditorBlueprintResources/StandardMacros.Gate` true :!label _label
    (:`Exit`
      (`self.InputPickUpEvent_Client`))))

(event `self.PickableArea.OnComponentBeginOverlap`
  (params (OverlappedComponent :type "PrimitiveComponent Object Reference") (OtherActor :type "Actor Object Reference") (OtherComp :type "PrimitiveComponent Object Reference") (OtherBodyIndex :type Integer) (bFromSweep :type Boolean) (SweepResult :type "HitResult Structure (by ref)"))
  (bind _asbp_third_person_character (cast `/Game/Werthy/Blueprints/BP_ThirdPersonCharacter` OtherActor))
  (`/Engine/EditorBlueprintResources/StandardMacros.IsValid` _asbp_third_person_character
    (:`Is Valid`
      (`/Game/Werthy/Blueprints/BP_ThirdPersonCharacter.SetInteractionObjectRefEvent` _asbp_third_person_character self true)
      (goto _label :!via `Open`))))

(event `InputPickUpEvent_Client`
  (`SceneComponent.SetVisibility` (`self.ColorfulWeapon`) false false))

(event `self.PickableArea.OnComponentEndOverlap`
  (params (OverlappedComponent :type "PrimitiveComponent Object Reference") (OtherActor :type "Actor Object Reference") (OtherComp :type "PrimitiveComponent Object Reference") (OtherBodyIndex :type Integer))
  (bind _asbp_third_person_character (cast `/Game/Werthy/Blueprints/BP_ThirdPersonCharacter` OtherActor))
  (`/Engine/EditorBlueprintResources/StandardMacros.IsValid` _asbp_third_person_character
    (:`Is Valid`
      (`/Game/Werthy/Blueprints/BP_ThirdPersonCharacter.SetInteractionObjectRefEvent` _asbp_third_person_character self false)
      (goto _label :!via `Close`))))

(fn `UserConstructionScript`)